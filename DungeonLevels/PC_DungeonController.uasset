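; Player controller for dungeon levels that handles pawn movement with a stun lock, player lives, spawning and HUD.
; Character selection opens a client widget and passes the choice through a server event to the game mode.
; First spawn possesses a new pawn and caches its stats, which respawns restore while lives remain; running out only prints Game Over.
; Client events build or regenerate the HUD, while update events feed health, mana, potion and currency displays.
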(event Custom|Client_Initialize
  (bind _returnvalue (UserInterface|CreateWidget "/Game/_Main/DungeonLevels/W_ClientCharacterSelect.W_ClientCharacterSelect_C"))
  (Variables|Default|SetClientCharacterSelect _returnvalue)
  (UserInterface|Viewport|AddtoViewport _returnvalue 0)
  (Input|SetInputModeUIOnly self _returnvalue "DoNotLock")
  (Variables|Default|SetbShowMouseCursor true)
  (Default|UpdateAvailableCharacters _returnvalue (Variables|Default|GetAvailable%20Characters)))

(event Custom|Client_UpdateCurrencyUI
  (params (Currency :type Integer))
  (Default|UpdateCurrency (Variables|Default|GetPlayerUI) Currency))

(event Custom|Client_LoadUI
  ;[1 1 1] Initializes the player and loads UI
  (if (Pawn|IsLocalPlayerController)
    (Variables|Default|GetPlayerUI
      (:then
        (CallFunction|ClientRegenerateUI))
      (:else
        (Utilities|FlowControl|Delay 0.35)
        (bind _returnvalue (UserInterface|CreateWidget "/Game/_Main/UI/PlayerUI.PlayerUI_C"))
        (bind _output_get (Variables|Default|SetPlayerUI _returnvalue))
        (UserInterface|Viewport|AddtoViewport _output_get 0)
        (Input|SetInputModeGameOnly self)
        (Variables|Default|SetbShowMouseCursor false)))))

(event Custom|Server_AssignCharacter
  (params (Character :type Integer))
  (Class|INTGameMode|GetSelectedClass(Message) (Game|GetGameMode) Character self))

(event Custom|Client_RegenerateUI
  ;[1 1 1] Initializes the player and loads UI
  (Widget|RemovefromParent (Variables|Default|GetPlayerUI))
  (Variables|Default|SetPlayerUI 0)
  (Utilities|FlowControl|Delay 0.35)
  (bind _returnvalue (UserInterface|CreateWidget "/Game/_Main/UI/PlayerUI.PlayerUI_C"))
  (bind _output_get (Variables|Default|SetPlayerUI _returnvalue))
  (UserInterface|Viewport|AddtoViewport _output_get 0)
  (Input|SetInputModeGameOnly self)
  (Variables|Default|SetbShowMouseCursor false))

(event EventUpdateCurrency
  (params (Currency :type Integer))
  (CallFunction|ClientUpdateCurrencyUI Currency))

(event EventMovementFrozen
  (params (State :type Boolean))
  ;[1 1 1] Interfaces/ UI Updates
  (Variables|Default|SetPlayerStunned State))

(event EventSavePlayerStats
  (params (Stats :type S%20Stats%20Structure))
  (Variables|Default|SetSavedStats Stats))

(event EventInitializePlayer
  ;[1 1 1] Initializes the player and loads UI
  (Utilities|FlowControl|Delay 0.2)
  (CallFunction|ClientLoadUI))

(event EventInitializeClient
  (params (AvailableCharacters :type Array%20of%20Booleans))
  (Variables|Default|SetAvailable%20Characters AvailableCharacters)
  (Utilities|FlowControl|Delay 1.0)
  (CallFunction|ClientInitialize))

(event EventAssignCharacter
  (params (Character :type Integer))
  (CallFunction|ServerAssignCharacter Character)
  (Widget|RemovefromParent (Variables|Default|GetClientCharacterSelect))
  (Input|SetInputModeGameOnly self)
  (Variables|Default|SetbShowMouseCursor false))

(event EventIncreaseLives
  ;[1 1 1] Interfaces/ UI Updates
  (Variables|Default|SetPlayerLives (+ (Variables|Default|GetPlayerLives) 1)))

(event EventDecreaseLives
  ;[1 1 1] Interfaces/ UI Updates
  (Variables|Default|SetPlayerLives (- (Variables|Default|GetPlayerLives) 1)))

(event EventPlayerRespawn
  (params (SpawnedLocation :type Vector :default "0, 0, 0") (PlayerClass :type BP%20Player%20Base%20Class%20Reference))
  (bind _returnvalue (Pawn|GetControlledPawn))
  ;[1 1 1] Respawns the player called from the Gamemode
  (Pawn|UnPossess)
  (if (> (Variables|Default|GetPlayerLives) 0)
    (bind _returnvalue_2 (Game|SpawnActorfromClass PlayerClass (Math|Transform|MakeTransform (+ SpawnedLocation "0, 0,150.000000") "0, 0, 0" "1,1,1") "AlwaysSpawn" 0 0))
    (Pawn|Possess _returnvalue_2)
    (Variables|Default|SetPlayerStunned false)
    (Variables|Default|SetPlayerPawn _returnvalue)
    (Class|INTPlayerCharacter|SetRespawnStats(Message) _returnvalue (Variables|Default|GetSavedStats))
    (Utilities|FlowControl|Delay 0.2)
    (CallFunction|InitializePlayer)
    (else
      (Development|PrintString "PC_DungeonController: Player has no more lives! Game Over"))))

(event EventUpdateHealthUI
  (params (CurrentHealth :type Float%20%28single-precision%29) (Percent :type Float%20%28single-precision%29))
  ;[1 1 1] Interfaces/ UI Updates
  (Default|UpdateHealthBar (Variables|Default|GetPlayerUI) CurrentHealth Percent))

(event EventUpdateManaUI
  (params (CurrentMana :type Float%20%28single-precision%29) (Percent :type Float%20%28single-precision%29))
  ;[1 1 1] Interfaces/ UI Updates
  (Default|UpdateManaBar (Variables|Default|GetPlayerUI) CurrentMana Percent))

(event EventUpdatePotionUI
  (params (isVisible :type Boolean))
  ;[1 1 1] Interfaces/ UI Updates
  (Default|UpdatePotion (Variables|Default|GetPlayerUI) isVisible))

(event EventPlayerFirstSpawn
  (params (SpawnLocation :type Vector :default "0, 0, 0") (Class :type BP%20Player%20Base%20Class%20Reference))
  (bind _returnvalue (Pawn|GetControlledPawn))
  ;[1 1 1] Spawns the player for the first time
  (bind _returnvalue_2 (Game|SpawnActorfromClass Class (Math|Transform|MakeTransform (+ SpawnLocation "0, 0,150.000000") "0, 0, 0" "1,1,1") "AlwaysSpawn" 0 0))
  (Pawn|Possess _returnvalue_2)
  (Variables|Default|SetPlayerStunned false)
  (Variables|Default|SetPlayerPawn _returnvalue)
  (bind _playerstats (Class|INTPlayerCharacter|GetInitialStats(Message) _returnvalue))
  (Variables|Default|SetSavedStats _playerstats)
  (Utilities|FlowControl|Delay 0.2)
  (CallFunction|InitializePlayer))

(event EventGetClass
  ;[1 1 1] Gets the Selected Class from Game Instance
  ;
  ; NOTE: Disconnect Selected Class for Test Levels
  (Class|INTGameInstance|GetPlayerClass(Message) (Game|GetGameInstance))
  (Class|INTGameMode|GetSelectedClass(Message) (Game|GetGameMode) 1 self))

(event Input|AxisEvents|InputAxisMoveForward
  (params (AxisValue :type Float%20%28single-precision%29))
  (bind _playerpawn (Variables|Default|GetPlayerPawn))
  ;[1 1 1] Player Movement
  (Variables|Default|GetPlayerPawn
    (:then
      (if (not (Variables|Default|GetPlayerStunned))
        (Pawn|Input|AddMovementInput _playerpawn (Math|Vector|GetForwardVector (Pawn|GetControlRotation _playerpawn :!class /Script/Engine.Pawn)) AxisValue false)))
    (:else)))

(event Input|AxisEvents|InputAxisMoveRight
  (params (AxisValue :type Float%20%28single-precision%29))
  (bind _playerpawn (Variables|Default|GetPlayerPawn))
  ;[1 1 1] Player Movement
  (Variables|Default|GetPlayerPawn
    (:then
      (if (not (Variables|Default|GetPlayerStunned))
        (Pawn|Input|AddMovementInput _playerpawn (Math|Vector|GetRightVector (Pawn|GetControlRotation _playerpawn :!class /Script/Engine.Pawn)) AxisValue false)))
    (:else)))

(fn ConstructionScript)

(fn GetSavedStats
  (return (Variables|Default|GetSavedStats)))