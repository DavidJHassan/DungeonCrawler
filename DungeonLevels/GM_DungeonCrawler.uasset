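; Dungeon crawler game mode that coordinates character class selection and first spawn for joining players.
; On login it tracks each controller, prompting the first local player for a class and sending other clients the character availability array.
; A selection marks an unclaimed character as taken and resolves its class.
; After a short delay, the requesting controller receives that class and the first-found PlayerStart's location for spawning.
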(event EventGetSelectedClass
  (params (Class :type Integer) (PC_DungeonCrontroller :type PC%20Dungeon%20Controller%20Object%20Reference))
  (bind _character (CallFunction|UpdateCharacters Class))
  (Utilities|FlowControl|Delay 1.0)
  (Class|INTPlayerController|PlayerFirstSpawn(Message) PC_DungeonCrontroller (Variables|Default|GetPlayerSpawnLocation) _character))

(event EventBeginPlay
  (bind _outactors (Actor|GetAllActorsOfClass "/Script/Engine.PlayerStart"))
  (bind _output_get (Variables|Default|SetStartingSpawns _outactors))
  (Variables|Default|SetPlayerSpawnLocation (Transformation|GetActorLocation (Utilities|Array|Get(acopy) _output_get))))

(event EventPostLogin
  (params (NewPlayer :type Player%20Controller%20Object%20Reference))
  (Utilities|Array|AddUnique (Variables|Default|GetConnectedPlayers) NewPlayer)
  (if (== (Game|GetPlayerController 0) NewPlayer)
    (Class|INTPlayerController|GetClass(Message) NewPlayer)
    (else
      (Class|INTPlayerController|InitializeClient(Message) NewPlayer (Variables|Default|GetAvailableCharacters)))))

(fn ConstructionScript)

(fn UpdateCharacters
  (params (SelectedCharacter :type Integer))
  (if (not (Utilities|Array|Get(acopy) (Variables|Default|GetAvailableCharacters) SelectedCharacter))
    (Utilities|Array|SetArrayElem (Variables|Default|GetAvailableCharacters) SelectedCharacter true)
    (return (Utilities|Array|Get(acopy) (Variables|Default|GetCharacters) SelectedCharacter))))