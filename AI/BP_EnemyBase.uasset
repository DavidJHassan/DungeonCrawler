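; Base enemy character for a networked game that chases a player, attacks, can be stunned and returns to its spawn point when it loses the target.
; AI MoveTo and distance checks loop chasing and montage attacks, with authority-only melee sphere overlaps or projectile spawns.
; Damage reduces struct-held health, with timer-driven damage over time and attached particles.
; Death multicasts ragdoll collision and an overridable animation, rolls potion or coin drops, then destroys the actor.
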(event Custom|ChasePlayer
  ;[1 1 1] Chase the Target
  (if (Variables|Default|GetinCombat)
    (AI|AIMoveTo self "0, 0, 0" (Variables|Default|GetPlayer%20Target) (Variables|Attack|GetAcceptance%20Radius) true
      (:OnSuccess
        (CallFunction|CheckAttackDistance))
      (:OnFail
        (CallFunction|ClearTarget)))))

(event Custom|ClearTarget
  ;[1 1 1] Clear Target and Reset Position
  (Variables|Default|SetinCombat false)
  (Actor|Tick|SetActorTickEnabled false)
  (Variables|Default|SetPlayer%20Target 0)
  (if (not (Variables|Default|GetIsDead))
    (AI|AIMoveTo self (CallFunction|FGetSpawnedLocation) 0 2e+01 false
      (:OnSuccess
        (bind _asbp_aicontroller (Utilities|Casting|CastToBP_AIController (Pawn|GetController)))
        (Default|ClearTarget _asbp_aicontroller))
      (:OnFail
        (Development|PrintString "BP_EnemyBase | ClearTarget: AI Move To Fail")))))

(event Custom|CheckAttackDistance
  ;[1 1 1] AI Attacking
  (if (and (not (Variables|Default|GetIsDead)) (not (Variables|Default|GetisStunned)))
    (bind _state (Class|INTPlayerCharacter|PlayerDeathState(Message) (Variables|Default|GetPlayer%20Target)))
    (if (not _state)
      (bind _output_get (Variables|Default|SetDistanceToPlayer (Transformation|GetDistanceTo (Variables|Default|GetPlayer%20Target))))
      (if (<= _output_get (Variables|Attack|GetAttackDistance))
        (CallFunction|FPlayAttackMontage)
        (Utilities|FlowControl|Delay (Variables|Attack|GetTimeBetweenAttacks))
        (CallFunction|CheckAttackDistance)
        (else
          (CallFunction|ChasePlayer)))
      (else
        (CallFunction|ClearTarget)))))

(event Custom|KillEnemy
  ;[1 1 1] Enemy Death Event
  (Variables|Default|SetIsDead true)
  (Pawn|Components|CharacterMovement|DisableMovement (Variables|Character|GetCharacterMovement))
  (CallFunction|ClearTarget)
  (CallFunction|MultiDeath)
  (Class|Pawn|DetachfromControllerPendingDestroy)
  (Class|CharacterMovementComponent|SetAvoidanceEnabled (Variables|Character|GetCharacterMovement) false)
  (if (Utilities|PercentageChance 6.0)
    (Game|SpawnActorfromClass "/Game/_Main/BP_PotionTest.BP_PotionTest_C" (Transformation|GetActorTransform) "AlwaysSpawn" 0 0)
    (elif (Utilities|PercentageChance 4e+01)
      (Game|SpawnActorfromClass "/Game/_Main/Currency/Currency_Coin.Currency_Coin_C" (Transformation|GetActorTransform) "AlwaysSpawn" 0 0)))
  (Utilities|FlowControl|Delay 15.0)
  (Actor|DestroyActor))

(event Custom|Multi_Death
  ;[1 1 1] Enemy Death Event
  (Collision|SetCollisionProfileName (Variables|Default|GetCapsuleComponent) "Ragdoll" true :!class /Script/Engine.PrimitiveComponent)
  (Components|Animation|SetAnimationMode (Variables|Character|GetMesh) "AnimationSingleNode")
  (CallFunction|DeathAnimation))

(event Custom|DeathAnimation
  ;[1 1 1] Overrides
)

(event Custom|AttachDOTParticle
  (params (DOT%20Class :type BP%20DOT%20Effect%20Base%20Class%20Reference) (Tick%20Amount :type Integer))
  ;[1 1 1] Damage Over Time
  (bind _returnvalue (Game|SpawnActorfromClass DOT%20Class (Transformation|GetActorTransform) "AlwaysSpawn" 0 Tick%20Amount 0))
  (Transformation|AttachComponentToComponent _returnvalue (Variables|Character|GetMesh) "Pelvis" "SnapToTarget" "SnapToTarget" "SnapToTarget" true))

(event Custom|DOTTimer
  ;[1 1 1] Damage Over Time
  (Game|Damage|ApplyDamage self (Variables|DOT|GetDOT) 0 0 "/Script/Engine.DamageType")
  (Utilities|FlowControl|Sequence
    (:then_0
      (if (<= (.CurrentHealth (Utilities|Struct|BreakS_Stats (Variables|Default|GetStats))) 0.0)
        (Utilities|Time|ClearandInvalidateTimerbyHandle (Variables|DOT|GetDOTHandle))))
    (:then_1
      (Variables|DOT|SetDOTCurrAmount (+ (Variables|DOT|GetDOTCurrAmount) 1))
      (if (== (Variables|DOT|GetDOTCurrAmount) (Variables|DOT|GetDOTNumTicks))
        (Utilities|Time|ClearandInvalidateTimerbyHandle (Variables|DOT|GetDOTHandle))))))

(event EventBeginPlay
  ;[1 1 1] Clear Target and Reset Position
  (CallFunction|FMovementState "NewEnumerator0")
  (CallFunction|AISpawnedLocation))

(event EventAIStunned
  (params (StunTime :type Float%20%28single-precision%29))
  ;[1 1 1] Enemy is Stunned
  (Actor|Tick|SetActorTickEnabled false)
  (CallFunction|MultiStunnedMontage (Variables|Character|GetMesh) (Variables|Default|GetStunnedMontage))
  (Variables|Default|SetisStunned true)
  (Utilities|FlowControl|Delay StunTime)
  (Actor|Tick|SetActorTickEnabled true)
  (Variables|Default|SetisStunned false))

(event EventDamageOverTime
  (params (DOT :type Float%20%28single-precision%29) (DamageTick :type Integer) (DOTClass :type BP%20DOT%20Effect%20Base%20Class%20Reference))
  ;[1 1 1] Damage Over Time
  (if (not (Variables|DOT|GetCurrentlyDOTted))
    (Variables|DOT|SetDOT DOT)
    (Variables|DOT|SetDOTNumTicks DamageTick)
    (bind _returnvalue (Utilities|Time|SetTimerbyEvent (delegate Custom|DOTTimer) 1.0))
    (Variables|DOT|SetDOTHandle _returnvalue)
    (CallFunction|AttachDOTParticle DOTClass (Variables|DOT|GetDOTNumTicks))))

(event Game|Damage|EventAnyDamage
  (params (Damage :type Float%20%28single-precision%29) (DamageType :type Damage%20Type%20Object%20Reference) (InstigatedBy :type Controller%20Object%20Reference) (DamageCauser :type Actor%20Object%20Reference))
  ;[1 1 1] Enemy Recieve Damage and Check if HP is 0 or Less and Kill the Enemy
  (bind _structout (Utilities|Struct|SetmembersinS_Stats (Variables|Default|GetStats) (- (.CurrentHealth (Utilities|Struct|BreakS_Stats (Variables|Default|GetStats))) Damage)))
  (if (<= (.CurrentHealth (Utilities|Struct|BreakS_Stats _structout)) 0.0)
    (CallFunction|KillEnemy)))

(event EventSetNewTarget
  (params (PlayerTarget :type Pawn%20Object%20Reference))
  ;[1 1 1] Set New Target
  (Variables|Default|GetPlayer%20Target
    (:then)
    (:else
      (bind _state (Class|INTPlayerCharacter|PlayerDeathState(Message) PlayerTarget))
      (if (not _state)
        (Variables|Default|SetPlayer%20Target PlayerTarget)
        (Variables|Default|SetinCombat true)
        (Actor|Tick|SetActorTickEnabled true)
        (CallFunction|FMovementState "NewEnumerator1")
        (CallFunction|ChasePlayer)))))

(event EventTick
  (params (DeltaSeconds :type Float%20%28single-precision%29))
  ;[1 1 1] Rotate Towards Target
  (Variables|Default|GetPlayer%20Target
    (:then
      (if (Variables|Default|GetinCombat)
        (Transformation|SetActorRotation (Math|Rotator|MakeRotator 0.0 0.0 (.yaw (Math|Rotator|FindLookatRotation (Transformation|GetActorLocation) (Transformation|GetActorLocation (Variables|Default|GetPlayer%20Target))))))))
    (:else
      (Actor|Tick|SetActorTickEnabled false)
      (CallFunction|ClearTarget))))

(event EventAIRangeAttack
  (bind _projectilespawnlocation (Variables|Default|GetProjectileSpawnLocation))
  ;[1 1 1] AI Attacking
  (Networking|SwitchHasAuthority
    (:Authority
      (Game|SpawnActorfromClass (Variables|Attack|GetProjectile) (Math|Transform|MakeTransform (Transformation|GetWorldLocation _projectilespawnlocation) (Transformation|GetWorldRotation _projectilespawnlocation) "1,1,1") "Undefined" self (Variables|Attack|GetProjectileDamage) (Variables|Attack|GetProjectileSpeed) 0))))

(event EventAIMeleeAttack
  ;[1 1 1] AI Attacking
  (Networking|SwitchHasAuthority
    (:Authority
      (bind _outactors (Collision|SphereOverlapActors (+ (Transformation|GetActorLocation) (* (Transformation|GetActorForwardVector) (Variables|Default|GetMeleeSphereDistance))) (Variables|Default|GetMeleeSphereSize) (Utilities|Array|MakeArray "ObjectTypeQuery3") "/Game/_Main/BP_PlayerBase.BP_PlayerBase_C"))
      (for _array_element _outactors
        (if (Actor|ActorHasTag _array_element "Player")
          (Game|Damage|ApplyDamage _array_element (Variables|Default|GetMeleeDamage) 0 self "/Script/Engine.DamageType")
          (bind _blocked (Class|INTPlayerCharacter|DidBlock?(Message) _array_element (Math|Vector|GetUnitDirection(Vector) (Transformation|GetActorLocation) (Transformation|GetActorLocation _array_element))))
          (if (not _blocked)
            (CallFunction|MultiParticleHit (Variables|MeleeHit|GetHitParticle) (+ (Transformation|GetActorLocation) (* (Transformation|GetActorForwardVector) (Variables|MeleeHit|GetHitParticleDistance))) (Variables|MeleeHit|GetHitParticleScale))))))))

(fn ConstructionScript
  (|CallParentFunction))

(fn FMovementState
  (params (State :type E_AIMovementState%20Enum :default "NewEnumerator0"))
  (bind _charactermovement (Variables|Character|GetCharacterMovement))
  (switch Utilities|FlowControl|Switch|SwitchonE_AIMovementState State
    (:NewEnumerator0
      (Variables|/Script/Engine.CharacterMovementComponent|SetMaxWalkSpeed _charactermovement 0.0))
    (:NewEnumerator1
      (Variables|/Script/Engine.CharacterMovementComponent|SetMaxWalkSpeed _charactermovement (Variables|Default|GetWalk%20Speed)))))

(fn FPlayAttackMontage
  (CallFunction|MultiPrimaryAttack (Variables|Character|GetMesh) (Variables|Default|GetAttackMontage) (CallFunction|FGetMontageSection) (Variables|Default|GetAttack%20Sound)))

(fn AIDeathCheck
  (return (Variables|Default|GetIsDead)))