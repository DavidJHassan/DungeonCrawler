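; Base vendor actor that players can interact with, exposing a vendor type and a list of upgrade items.
; A sphere trigger, handled only on the server, turns the interactable message on for overlapping Player-tagged actors, passing itself as the target, and off when they leave.
; Simple getters return the interact type, vendor type and upgrade items, while purchase logic lives outside this Blueprint.
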(event OnComponentBeginOverlap(Sphere)
  (params (OverlappedComponent :type Primitive%20Component%20Object%20Reference) (OtherActor :type Actor%20Object%20Reference) (OtherComp :type Primitive%20Component%20Object%20Reference) (OtherBodyIndex :type Integer) (bFromSweep :type Boolean) (SweepResult :type Hit%20Result%20Structure%20%28by%20ref%29))
  (Networking|SwitchHasAuthority
    (:Authority
      (if (Actor|ActorHasTag OtherActor "Player")
        (Class|INTPlayerCharacter|SetInteractable(Message) OtherActor true self)))))

(event OnComponentEndOverlap(Sphere)
  (params (OverlappedComponent :type Primitive%20Component%20Object%20Reference) (OtherActor :type Actor%20Object%20Reference) (OtherComp :type Primitive%20Component%20Object%20Reference) (OtherBodyIndex :type Integer))
  (Networking|SwitchHasAuthority
    (:Authority
      (if (Actor|ActorHasTag OtherActor "Player")
        (Class|INTPlayerCharacter|SetInteractable(Message) OtherActor false)))))

(fn ConstructionScript)

(fn GetInteractType
  (return (Variables|Default|GetInteractType)))

(fn GetVendorItems
  (return (Variables|Default|GetUpgradeItems)))

(fn GetVendorType
  (return (Variables|Default|GetVenderType)))