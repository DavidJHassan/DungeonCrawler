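; Base character Blueprint that provides shared combat presentation and state, with hooks for both AI and player death.
; Multi_ events, named as multicasts, play attack, stun and generic montages, hit and voice sounds, and hit particles, with attack sound timed by a montage notify.
; After a short BeginPlay delay it caches controller, spawn location and AnimInstance, which receives the death message.
; Helper functions expose cached references, blocking state and a random attack montage section.
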(event Custom|Multi_PrimaryAttack
  (params (InSkeletalMeshComponent :type Skeletal%20Mesh%20Component%20Object%20Reference) (MontageToPlay :type Anim%20Montage%20Object%20Reference) (StartingSection :type Name) (AttackSound :type Sound%20Base%20Object%20Reference))
  (Animation|Montage|PlayMontage InSkeletalMeshComponent MontageToPlay 1.0 0.0 StartingSection
    (:OnNotifyBegin
      (Audio|PlaySoundatLocation AttackSound (Transformation|GetActorLocation) "0, 0, 0" 1.0 1.0 0.0 0 0 0))))

(event Custom|Multi_PlayHitSound
  (params (Location :type Vector) (Sound :type Sound%20Base%20Object%20Reference))
  (Audio|PlaySoundatLocation Sound Location "0, 0, 0" 1.0 1.0 0.0 0 0 0))

(event Custom|Multi_PlayerDead
  (Class|INTAnimBP|SetDead(Message) (Variables|Default|GetAnimInstance)))

(event Custom|Multi_StunnedMontage
  (params (InSkeletalMeshComponent :type Skeletal%20Mesh%20Component%20Object%20Reference) (MontageToPlay :type Anim%20Montage%20Object%20Reference))
  (Animation|Montage|PlayMontage InSkeletalMeshComponent MontageToPlay))

(event Custom|Multi_ParticleHit
  (params (EmitterTemplate :type Particle%20System%20Object%20Reference) (Location :type Vector) (Scale :type Vector))
  (Effects|SpawnEmitteratLocation EmitterTemplate Location "0, 0, 0" Scale))

(event Custom|Multi_PlayAnimation
  (params (InSkeletalMeshComponent :type Skeletal%20Mesh%20Component%20Object%20Reference) (MontageToPlay :type Anim%20Montage%20Object%20Reference) (StartingSection :type Name))
  (Animation|Montage|PlayMontage InSkeletalMeshComponent MontageToPlay))

(event Custom|AISpawnedLocation
  (Variables|Default|SetSpawnedLocation (Transformation|GetActorLocation)))

(event Custom|Multi_VoiceSound
  (params (Sound :type Sound%20Base%20Object%20Reference) (Location :type Vector))
  (Audio|PlaySoundatLocation Sound Location "0, 0, 0" 1.0 1.0 0.0 0 0 0))

(event EventBeginPlay
  (Utilities|FlowControl|Delay 0.5)
  (Variables|Default|SetControllerRef (Pawn|GetController))
  (Variables|Default|SetSpawnedLocation (Transformation|GetActorLocation))
  (Variables|Default|SetAnimInstance (Components|SkeletalMesh|GetAnimInstance (Variables|Character|GetMesh))))

(fn ConstructionScript)

(fn FGetMontageSection
  (bind _attacksections (Variables|Default|GetAttackSections))
  (return (Utilities|Array|Get(acopy) _attacksections (Math|Random|RandomIntegerinRange 0 (- (Utilities|Array|Length _attacksections) 1)))))

(fn FGetSpawnedLocation
  (return (Variables|Default|GetSpawnedLocation)))

(fn FGetAnimInstance
  (return (Variables|Default|GetAnimInstance)))

(fn FBlocking
  (params (State :type Boolean))
  (if State
    (Variables|Default|SetBlocking true)
    (else
      (Variables|Default|SetBlocking false))))

(fn FIsBlocking
  (return (Variables|Default|GetBlocking)))