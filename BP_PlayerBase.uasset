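; Base multiplayer player character that provides input, stats, potions, damage, death and vendor upgrades for child classes.
; Inputs call server events, with attacks, abilities and upgrade data left as stubs for children to override.
; Health, mana, potion and currency changes reach the UI through the player controller, which also saves stats and respawns the player on death.
; Interacting with vendors builds Health, Attack or Defense shop widgets priced against currency.
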(event Custom|Server_PrimaryAttack
  ;[1 1 1] Attack Overrides
)

(event Custom|Server_AbilityThree
  ;[1 1 1] Attack Overrides
)

(event Custom|Client_UpdatePotionUI
  (params (isVisible :type Boolean))
  ;[1 1 1] Update UI
  (Class|INTPlayerController|UpdatePotionUI(Message) (Variables|Default|GetControllerRef) isVisible))

(event Custom|Server_AbilityDash
  ;[1 1 1] Attack Overrides
)

(event Custom|Client_ReloadVendorWidget
  (params (Selection :type E_VendorType%20Enum :default "NewEnumerator0"))
  (Utilities|FlowControl|Delay 0.2)
  (switch Utilities|FlowControl|Switch|SwitchonE_VendorType Selection
    (:NewEnumerator0
      (CallFunction|FHealthVendorWidget))
    (:NewEnumerator1
      (CallFunction|FAttackVendorWidget))
    (:NewEnumerator2
      (CallFunction|FDefenseVendorWidget))))

(event Custom|Server_KillPlayer
  (bind _controllerref (Variables|Default|GetControllerRef))
  (bind _controllerref_2 (Variables|Default|GetControllerRef))
  ;[1 1 1] Player Death/ Respawn
  (if (not (Variables|Default|GetIsDead))
    (Variables|Default|SetIsDead true)
    (CallFunction|MultiPlayerDead)
    (CallFunction|MultiVoiceSound (Variables|Default|GetVoiceDeath) (Transformation|GetActorLocation))
    (Class|INTPlayerController|MovementFrozen(Message) _controllerref_2 true)
    (Class|INTPlayerController|SavePlayerStats(Message) _controllerref_2 (Variables|Default|GetStats))
    (Class|INTPlayerController|DecreaseLives(Message) _controllerref)
    (Utilities|FlowControl|Delay 5.0)
    (Class|INTPlayerController|PlayerRespawn(Message) _controllerref (CallFunction|FGetSpawnedLocation) (Variables|Default|GetPlayerClass))
    (Utilities|FlowControl|Delay 0.2)
    (Actor|DestroyActor)))

(event Custom|Server_UsePotion
  (bind _stats (Variables|Default|GetStats))
  ;[1 1 1] Potion Logic
  (if (Variables|Default|GetHasPotion)
    (bind _structout (Utilities|Struct|SetmembersinS_Stats _stats (Utilities|Struct|BreakS_Stats _stats)))
    (Variables|Default|SetHasPotion false)
    (CallFunction|ClientUpdateHealthUI (Utilities|Struct|BreakS_Stats _structout))
    (CallFunction|ClientUpdatePotionUI false)))

(event Custom|Client_UpdateHealthUI
  (params (CurrentHealth :type Float%20%28single-precision%29))
  ;[1 1 1] Update UI
  (Class|INTPlayerController|UpdateHealthUI(Message) (Variables|Default|GetControllerRef) CurrentHealth (/ CurrentHealth (.MaxHealth (Utilities|Struct|BreakS_Stats (Variables|Default|GetStats))))))

(event Custom|Client_UpdateManaUI
  (params (CurrentMana :type Float%20%28single-precision%29))
  ;[1 1 1] Update UI
  (Class|INTPlayerController|UpdateManaUI(Message) (Variables|Default|GetControllerRef) CurrentMana (/ CurrentMana (.MaxMana (Utilities|Struct|BreakS_Stats (Variables|Default|GetStats))))))

(event Custom|Server_AbilityOne
  ;[1 1 1] Attack Overrides
)

(event Custom|Server_AbilityTwo
  ;[1 1 1] Attack Overrides
)

(event Custom|Server_UpgradeSkills
  (params (Selection :type E_UpgradeableSkills%20Enum :default "NewEnumerator0") (Cost :type Integer))
  (bind _stats (Variables|Default|GetStats))
  (switch Utilities|FlowControl|Switch|SwitchonE_UpgradeableSkills Selection
    (:NewEnumerator0
      (bind _result (Math|Integer|IncrementInt (Variables|AbilityLevels|GetHealthPool))
        (:%20%20
          (Utilities|Struct|SetmembersinS_Stats _stats _result)
          (bind _new_amount (CallFunction|FUpgradeSkill "NewEnumerator0" Cost))
          (CallFunction|ClientUpdateHealthUI _new_amount))))
    (:NewEnumerator1
      (bind _result_2 (Math|Integer|IncrementInt (Variables|AbilityLevels|GetManaPool))
        (:%20%20
          (Utilities|Struct|SetmembersinS_Stats _stats _result_2)
          (bind _new_amount_2 (CallFunction|FUpgradeSkill "NewEnumerator1" Cost))
          (CallFunction|ClientUpdateManaUI _new_amount_2))))
    (:NewEnumerator2
      (bind _result_3 (Math|Integer|IncrementInt (Variables|AbilityLevels|GetPrimaryAttackLevel))
        (:%20%20
          (Utilities|Struct|SetmembersinS_Stats _stats _result_3)
          (CallFunction|FUpgradeSkill "NewEnumerator2" Cost))))
    (:NewEnumerator3
      (bind _result_4 (Math|Integer|IncrementInt (Variables|AbilityLevels|GetAbilityOneLevel))
        (:%20%20
          (Utilities|Struct|SetmembersinS_Stats _stats _result_4)
          (CallFunction|FUpgradeSkill "NewEnumerator3" Cost))))
    (:NewEnumerator4
      (bind _result_5 (Math|Integer|IncrementInt (Variables|AbilityLevels|GetAbilityTwoLevel))
        (:%20%20
          (Utilities|Struct|SetmembersinS_Stats _stats _result_5)
          (CallFunction|FUpgradeSkill "NewEnumerator4" Cost))))
    (:NewEnumerator5
      (bind _result_6 (Math|Integer|IncrementInt (Variables|AbilityLevels|GetAbilityThreeLevel))
        (:%20%20
          (Utilities|Struct|SetmembersinS_Stats _stats _result_6)
          (CallFunction|FUpgradeSkill "NewEnumerator5" Cost))))))

(event Custom|UpdatePlayerMovement
  (params (State :type Boolean))
  (if State
    (Class|INTPlayerController|MovementFrozen(Message) (Variables|Default|GetControllerRef) true)
    (elif (not (Variables|Default|GetIsDead))
      (Class|INTPlayerController|MovementFrozen(Message) (Variables|Default|GetControllerRef) false))))

(event EventAddPotion
  ;[1 1 1] Potion Logic
  (Variables|Default|SetHasPotion true)
  (CallFunction|ClientUpdatePotionUI true))

(event EventAddCurrency
  (params (CurrencyToAdd :type Integer))
  (bind _stats (Variables|Default|GetStats))
  (bind _structout (Utilities|Struct|SetmembersinS_Stats _stats (+ (Utilities|Struct|BreakS_Stats _stats) CurrencyToAdd)))
  (Class|INTPlayerController|UpdateCurrency(Message) (Variables|Default|GetControllerRef) (Utilities|Struct|BreakS_Stats _structout)))

(event EventSetInteractable
  (params (State :type Boolean) (Inertactable :type Actor%20Object%20Reference))
  ;[1 1 1] Interactable Event Triggered
  (if State
    (Variables|Default|SetInteracteable Inertactable)
    (else
      (Variables|Default|SetInteracteable 0))))

(event Game|Damage|EventAnyDamage
  (params (Damage :type Float%20%28single-precision%29) (DamageType :type Damage%20Type%20Object%20Reference) (InstigatedBy :type Controller%20Object%20Reference) (DamageCauser :type Actor%20Object%20Reference))
  ;[1 1 1] Damage Event
  (if (not (Variables|Default|GetisInvincible))
    (bind _structout (Utilities|Struct|SetmembersinS_Stats (Variables|Default|GetStats) (- (Utilities|Struct|BreakS_Stats (Variables|Default|GetStats)) Damage)))
    (CallFunction|ClientUpdateHealthUI (.CurrentHealth (Utilities|Struct|BreakS_Stats _structout)))
    (CallFunction|MultiVoiceSound (Variables|Default|GetVoicePain) (Transformation|GetActorLocation))
    (if (<= (Utilities|Struct|BreakS_Stats (Variables|Default|GetStats)) 0.0)
      (CallFunction|ServerKillPlayer))))

(event EventCloseWidgets
  (bind _returnvalue (Game|GetPlayerController 0))
  (Input|SetInputModeGameOnly _returnvalue)
  (Variables|/Script/Engine.PlayerController|SetbShowMouseCursor _returnvalue false))

(event EventUpdateVendorDescription
  (params (Description :type Text))
  (bind _vendorwidget (Variables|Default|GetVendorWidget)
    (:then
      (Default|UpdateDescription _vendorwidget Description))
    (:else)))

(event EventSetRespawnStats
  (params (Stats :type S%20Stats%20Structure))
  (bind (_maxhealth _maxmana _currency _healthpool _manapool _primaryattacklevel _ability1level _ability2level _ability3level) (Utilities|Struct|BreakS_Stats Stats))
  ;[1 1 1] Sets the Stored Stats from the Player Controller to the New Spawned Class
  (bind _structout (Utilities|Struct|SetmembersinS_Stats (Variables|Default|GetStats) _maxhealth _maxhealth _maxmana _maxmana _currency _healthpool _manapool _primaryattacklevel _ability1level _ability2level _ability3level))
  (CallFunction|FLoadStats _structout))

(event EventUpgradeSkill
  (params (Skill :type E_UpgradeableSkills%20Enum :default "NewEnumerator0") (Cost :type Integer))
  (CallFunction|ServerUpgradeSkills Skill Cost))

(event Input|ActionEvents|InputActionPrimaryAttack
  (params (Key :type Key%20Structure :default "None"))
  ;[1 1 1] Player Abilities/Inputs
  (:Pressed
    (if (not (Variables|Default|GetIsDead))
      (if (not (Variables|Default|GetCurrentlyAttacking))
        (CallFunction|ServerPrimaryAttack)))))

(event Input|ActionEvents|InputActionDash
  (params (Key :type Key%20Structure :default "None"))
  ;[1 1 1] Player Abilities/Inputs
  (:Pressed
    (if (not (Variables|Default|GetIsDead))
      (CallFunction|ServerAbilityDash))))

(event Input|ActionEvents|InputActionUsePotion
  (params (Key :type Key%20Structure :default "None"))
  ;[1 1 1] Potion Logic
  (:Pressed
    (CallFunction|ServerUsePotion)))

(event Input|ActionEvents|InputActionAbilityOne
  (params (Key :type Key%20Structure :default "None"))
  ;[1 1 1] Player Abilities/Inputs
  (:Pressed
    (if (not (Variables|Default|GetIsDead))
      (if (not (Variables|Default|GetCurrentlyAttacking))
        (CallFunction|ServerAbilityOne)))))

(event Input|ActionEvents|InputActionInteract
  (params (Key :type Key%20Structure :default "None"))
  ;[1 1 1] Interactable Event Triggered
  (:Pressed
    (bind _interacteable (Variables|Default|GetInteracteable)
      (:then
        (bind _interacttype (Class|INTInteract|GetInteractType(Message) _interacteable))
        (switch Utilities|FlowControl|Switch|SwitchonE_Interactable _interacttype
          (:NewEnumerator0
            (CallFunction|FVendors (Variables|Default|GetInteracteable)))))
      (:else))))

(event Input|ActionEvents|InputActionAbilityTwo
  (params (Key :type Key%20Structure :default "None"))
  ;[1 1 1] Player Abilities/Inputs
  (:Pressed
    (if (not (Variables|Default|GetIsDead))
      (if (not (Variables|Default|GetCurrentlyAttacking))
        (CallFunction|ServerAbilityTwo)))))

(event Input|ActionEvents|InputActionAbilityThree
  (params (Key :type Key%20Structure :default "None"))
  ;[1 1 1] Player Abilities/Inputs
  (:Pressed
    (if (not (Variables|Default|GetIsDead))
      (if (not (Variables|Default|GetCurrentlyAttacking))
        (CallFunction|ServerAbilityThree)))))

(fn ConstructionScript)

(fn FUpdateMana
  (params (ManaCost :type Float%20%28single-precision%29))
  (bind _stats (Variables|Default|GetStats))
  (bind _structout (Utilities|Struct|SetmembersinS_Stats _stats (- (.CurrentMana (Utilities|Struct|BreakS_Stats _stats)) ManaCost)))
  (return (.CurrentMana (Utilities|Struct|BreakS_Stats _structout))))

(fn FVendors
  (params (Object :type Actor%20Object%20Reference))
  (bind _vendortype (Class|INTVendor|GetVendorType(Message) Object))
  (switch Utilities|FlowControl|Switch|SwitchonE_VendorType _vendortype
    (:NewEnumerator0
      (CallFunction|FHealthVendorWidget))
    (:NewEnumerator1
      (CallFunction|FAttackVendorWidget))
    (:NewEnumerator2
      (CallFunction|FDefenseVendorWidget))))

(fn FGetHealthPool
  ;[1 0 0.007957] Overridden in Child Class
  (return false "" 0 ""))

(fn FGetManaPool
  ;[1 0.8114 0] Overriden in child class
  (return false "" 0 ""))

(fn FHealthVendorWidget
  (bind (_generate _name _cost _description) (CallFunction|FGetHealthPool))
  (bind (_generate_2 _name_2 _cost_2 _description_2) (CallFunction|FGetManaPool))
  (bind _returnvalue (Game|GetPlayerController 0))
  (bind _stats (Variables|Default|GetStats))
  (bind _stats_2 (Variables|Default|GetStats))
  (bind _currency (Utilities|Struct|BreakS_Stats _stats))
  (bind _currency_2 (Utilities|Struct|BreakS_Stats _stats_2))
  (bind _vendorwidget (Variables|Default|GetVendorWidget)
    (:then
      (Widget|RemovefromParent _vendorwidget))
    (:else
      _))
  (bind _returnvalue_2 (UserInterface|CreateWidget "/Game/_Main/Vendors/W_VendorWidget.W_VendorWidget_C" (Game|GetPlayerController 0)))
  (Variables|Default|SetVendorWidget _returnvalue_2)
  (UserInterface|Viewport|AddtoViewport _returnvalue_2 0)
  (Input|SetInputModeUIOnly _returnvalue (Variables|Default|GetVendorWidget) "DoNotLock")
  (Variables|/Script/Engine.PlayerController|SetbShowMouseCursor _returnvalue true)
  (bind _upgradeitems (Class|INTVendor|GetVendorItems(Message) (Variables|Default|GetInteracteable)))
  (for (_ _array_index) _upgradeitems
    (switch int _array_index
      (:0
        (Default|PopulateVendorItems (Variables|Default|GetVendorWidget) _generate (Game|GetPlayerController 0) _name _cost (>= _currency_2 _cost) _description _currency_2 "NewEnumerator0"))
      (:1
        (Default|PopulateVendorItems (Variables|Default|GetVendorWidget) _generate_2 (Game|GetPlayerController 0) _name_2 _cost_2 (>= _currency _cost_2) _description_2 _currency "NewEnumerator1")))))

(fn FUpgradeSkill
  (params (SkillToUpgrade :type E_UpgradeableSkills%20Enum :default "NewEnumerator0") (Cost :type Integer))
  (return 0.0))

(fn FAttackVendorWidget
  (bind (_generate _name _cost _description _skill) (CallFunction|FAttackUpgrades 3))
  (bind (_generate_2 _name_2 _cost_2 _description_2 _skill_2) (CallFunction|FAttackUpgrades))
  (bind (_generate_3 _name_3 _cost_3 _description_3 _skill_3) (CallFunction|FAttackUpgrades 1))
  (bind (_generate_4 _name_4 _cost_4 _description_4 _skill_4) (CallFunction|FAttackUpgrades 2))
  (bind _returnvalue (Game|GetPlayerController 0))
  (bind _stats (Variables|Default|GetStats))
  (bind _stats_2 (Variables|Default|GetStats))
  (bind _stats_3 (Variables|Default|GetStats))
  (bind _stats_4 (Variables|Default|GetStats))
  (bind _currency (Utilities|Struct|BreakS_Stats _stats_4))
  (bind _currency_2 (Utilities|Struct|BreakS_Stats _stats))
  (bind _currency_3 (Utilities|Struct|BreakS_Stats _stats_2))
  (bind _currency_4 (Utilities|Struct|BreakS_Stats _stats_3))
  (bind _vendorwidget (Variables|Default|GetVendorWidget)
    (:then
      (Widget|RemovefromParent _vendorwidget))
    (:else
      _))
  (bind _returnvalue_2 (UserInterface|CreateWidget "/Game/_Main/Vendors/W_VendorWidget.W_VendorWidget_C" (Game|GetPlayerController 0)))
  (Variables|Default|SetVendorWidget _returnvalue_2)
  (UserInterface|Viewport|AddtoViewport _returnvalue_2 0)
  (Input|SetInputModeUIOnly _returnvalue (Variables|Default|GetVendorWidget) "DoNotLock")
  (Variables|/Script/Engine.PlayerController|SetbShowMouseCursor _returnvalue true)
  (for (_ _array_index) (Variables|AbilityLevels|GetNumberOfAttacks)
    (switch int _array_index
      (:0
        (Default|PopulateVendorItems (Variables|Default|GetVendorWidget) _generate_2 (Game|GetPlayerController 0) _name_2 _cost_2 (>= _currency_4 _cost_2) _description_2 _currency_4 _skill_2))
      (:1
        (Default|PopulateVendorItems (Variables|Default|GetVendorWidget) _generate_3 (Game|GetPlayerController 0) _name_3 _cost_3 (>= _currency _cost_3) _description_3 _currency _skill_3))
      (:2
        (Default|PopulateVendorItems (Variables|Default|GetVendorWidget) _generate_4 (Game|GetPlayerController 0) _name_4 _cost_4 (>= _currency_2 _cost_4) _description_4 _currency_2 _skill_4))
      (:3
        (Default|PopulateVendorItems (Variables|Default|GetVendorWidget) _generate (Game|GetPlayerController 0) _name _cost (>= _currency_3 _cost) _description _currency_3 _skill)))))

(fn FAttackUpgrades
  (params (SkillNumber :type Integer))
  ;[1 0.1717 0] Overriden in child class
  (return false "" 0 "" "NewEnumerator0"))

(fn FDefenseVendorWidget
  (bind (_generate _name _cost _description _skill) (CallFunction|FDefenseUpgrades 3))
  (bind (_generate_2 _name_2 _cost_2 _description_2 _skill_2) (CallFunction|FDefenseUpgrades))
  (bind (_generate_3 _name_3 _cost_3 _description_3 _skill_3) (CallFunction|FDefenseUpgrades 1))
  (bind (_generate_4 _name_4 _cost_4 _description_4 _skill_4) (CallFunction|FDefenseUpgrades 2))
  (bind _returnvalue (Game|GetPlayerController 0))
  (bind _stats (Variables|Default|GetStats))
  (bind _stats_2 (Variables|Default|GetStats))
  (bind _stats_3 (Variables|Default|GetStats))
  (bind _stats_4 (Variables|Default|GetStats))
  (bind _currency (Utilities|Struct|BreakS_Stats _stats_4))
  (bind _currency_2 (Utilities|Struct|BreakS_Stats _stats))
  (bind _currency_3 (Utilities|Struct|BreakS_Stats _stats_2))
  (bind _currency_4 (Utilities|Struct|BreakS_Stats _stats_3))
  (bind _vendorwidget (Variables|Default|GetVendorWidget)
    (:then
      (Widget|RemovefromParent _vendorwidget))
    (:else
      _))
  (bind _returnvalue_2 (UserInterface|CreateWidget "/Game/_Main/Vendors/W_VendorWidget.W_VendorWidget_C" (Game|GetPlayerController 0)))
  (Variables|Default|SetVendorWidget _returnvalue_2)
  (UserInterface|Viewport|AddtoViewport _returnvalue_2 0)
  (Input|SetInputModeUIOnly _returnvalue (Variables|Default|GetVendorWidget) "DoNotLock")
  (Variables|/Script/Engine.PlayerController|SetbShowMouseCursor _returnvalue true)
  (for (_ _array_index) (Variables|AbilityLevels|GetNumberOfDefenseAbilities)
    (switch int _array_index
      (:0
        (Default|PopulateVendorItems (Variables|Default|GetVendorWidget) _generate_2 (Game|GetPlayerController 0) _name_2 _cost_2 (>= _currency_4 _cost_2) _description_2 _currency_4 _skill_2))
      (:1
        (Default|PopulateVendorItems (Variables|Default|GetVendorWidget) _generate_3 (Game|GetPlayerController 0) _name_3 _cost_3 (>= _currency _cost_3) _description_3 _currency _skill_3))
      (:2
        (Default|PopulateVendorItems (Variables|Default|GetVendorWidget) _generate_4 (Game|GetPlayerController 0) _name_4 _cost_4 (>= _currency_2 _cost_4) _description_4 _currency_2 _skill_4))
      (:3
        (Default|PopulateVendorItems (Variables|Default|GetVendorWidget) _generate (Game|GetPlayerController 0) _name _cost (>= _currency_3 _cost) _description _currency_3 _skill)))))

(fn FDefenseUpgrades
  (params (SkillNumber :type Integer))
  ;[1 0.1717 0] Overriden in child class
  (return false "" 0 "" "NewEnumerator0"))

(fn FUpdateCurrency
  (params (Cost :type Integer))
  (bind _stats (Variables|Default|GetStats))
  (bind _structout (Utilities|Struct|SetmembersinS_Stats _stats (- (Utilities|Struct|BreakS_Stats _stats) Cost)))
  (Class|INTPlayerController|UpdateCurrency(Message) (Variables|Default|GetControllerRef) (Utilities|Struct|BreakS_Stats _structout)))

(fn FLoadStats
  (params (Stats :type S%20Stats%20Structure))
  (bind (_healthpool _manapool _primaryattacklevel _ability1level _ability2level _ability3level) (Utilities|Struct|BreakS_Stats Stats))
  (Variables|AbilityLevels|SetHealthPool _healthpool)
  (Variables|AbilityLevels|SetManaPool _manapool)
  (Variables|AbilityLevels|SetPrimaryAttackLevel _primaryattacklevel)
  (Variables|AbilityLevels|SetAbilityOneLevel _ability1level)
  (Variables|AbilityLevels|SetAbilityTwoLevel _ability2level)
  (Variables|AbilityLevels|SetAbilityThreeLevel _ability3level))

(fn CheckforPotion
  (return (Variables|Default|GetHasPotion)))

(fn DidBlock?
  (params (UnitDirection :type Vector :default "0, 0, 0"))
  (return false))

(fn GetInitialStats
  (return (Variables|Default|GetStats)))

(fn IsPlayerInvincible
  (return (Variables|Default|GetisInvincible)))

(fn PlayerDeathState
  (return (Variables|Default|GetIsDead)))