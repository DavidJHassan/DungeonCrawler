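; Player controller for the main menu: it creates the menu widget, handles character selection and starts, hosts or joins games.
; Gamepad bottom-button presses route by the active widget enum to the menu border or game start.
; Highlight and select events drive spotlights and montages on CharacterSelect actors, storing the chosen class in the GameInstance alongside the player name.
; Hosting creates an advanced session and opens Level1 as listen server; joining uses session results or IP.
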(event Custom|CharacterHighlighted
  (params (Character :type E_CharacterSelect%20Enum :default "NewEnumerator0"))
  (for _array_element (Variables|Default|GetCharacterSelects)
    (if (== (Variables|/Game/_Main/CharacterSelect.CharacterSelect_C|GetCharacterSelect _array_element) Character)
      (Default|SpotlightSwitch _array_element true)
      (else
        (Default|SpotlightSwitch _array_element false)))))

(event Custom|CharacterSelected
  (params (Character :type E_CharacterSelect%20Enum :default "NewEnumerator0") (Class :type BP%20Player%20Base%20Class%20Reference))
  (bind _output_get (Variables|Default|SetSelectedClass Class))
  (Class|INTGameInstance|StoreSelectedClass(Message) (Game|GetGameInstance) _output_get)
  (for _array_element (Variables|Default|GetCharacterSelects)
    (if (== (Variables|/Game/_Main/CharacterSelect.CharacterSelect_C|GetCharacterSelect _array_element) Character)
      (Default|CharacterSelected _array_element Character)
      (else
        (Default|StopMontage _array_element)))))

(event Custom|StartGame
  (Game|OpenLevel(byName) "Level1"))

(event Custom|HostGame
  (params (ServerName :type Text) (HostClass :type Integer))
  (Class|INTGameInstance|StoreSelectedClass(Message) (Game|GetGameInstance) 0 HostClass)
  (|AdvancedSession (Utilities|Array|MakeArray (Class|AdvancedSessionsLibrary|MakeLiteralSessionPropertyString "ServerName" (Utilities|String|ToString(Text) ServerName))) self 4 0 false true false true true false false false true
    (:OnSuccess
      (Game|OpenLevel(byName) "Level1" true "?listen"))
    (:OnFailure
      (Development|PrintString "PC_MainMenu: Failed to host session" true true "(R=1.000000,G=0.329324,B=0.000000,A=1.000000)" 1e+01))))

(event Custom|JoinIP
  (params (IP :type String))
  (Development|ExecuteConsoleCommand (Utilities|String|Append "open " IP) self))

(event Custom|JoinServer
  (params (SearchResult :type Blueprint%20Session%20Result%20Structure%20%28by%20ref%29))
  (|JoinSession (Game|GetPlayerController 0) SearchResult
    (:OnFailure
      (Development|PrintString "PC_MainMenu: Failed to join session" true true "(R=1.000000,G=0.322247,B=0.000000,A=1.000000)" 1e+01))))

(event EventBeginPlay
  (Utilities|FlowControl|Sequence
    (:then_0
      (Input|DisableInput 0)
      (bind _returnvalue (UserInterface|CreateWidget "/Game/_Main/MainMenu/W_MainMenu.W_MainMenu_C"))
      (bind _output_get (Variables|Default|SetMainMenu _returnvalue))
      (UserInterface|Viewport|AddtoViewport _output_get 0)
      (Utilities|FlowControl|Delay 4.0)
      (Input|SetInputModeGameandUI self (Variables|/Game/_Main/MainMenu/W_MainMenu.W_MainMenu_C|GetW_MainMenuBorder (Variables|Default|GetMainMenu)) "DoNotLock" true)
      (Variables|Default|SetbShowMouseCursor true)
      (Input|EnableInput 0)
      (bind _outactors (Actor|GetAllActorsOfClass "/Game/_Main/CharacterSelect.CharacterSelect_C"))
      (Variables|Default|SetCharacterSelects _outactors))
    (:then_1
      (Utilities|UpdateButton (Variables|/Game/_Main/MainMenu/W_MainMenuBorder.W_MainMenuBorder_C|GetNewGameBTN (Variables|/Game/_Main/MainMenu/W_MainMenu.W_MainMenu_C|GetW_MainMenuBorder (Variables|Default|GetMainMenu))) "(X=1.200000,Y=1.200000)" "(R=1.000000,G=0.000000,B=0.000000,A=1.000000)"))
    (:then_2
      (Utilities|FlowControl|Delay 0.5)
      (bind _output_get_2 (Variables|Default|SetPlayerName (Utilities|Text|ToText(String) (Class|AdvancedSessionsLibrary|GetPlayerName self))))
      (Class|INTGameInstance|StorePlayerName(Message) (Game|GetGameInstance) _output_get_2))))

(event Input|GamepadEvents|GamepadFaceButtonBottom
  (params (Key :type Key%20Structure :default "None"))
  (:Pressed
    (switch Utilities|FlowControl|Switch|SwitchonE_InWidget (Variables|Default|GetInWidget)
      (:NewEnumerator4
        (Default|BottomButtonPressed (Variables|/Game/_Main/MainMenu/W_MainMenu.W_MainMenu_C|GetW_MainMenuBorder (Variables|Default|GetMainMenu))))
      (:NewEnumerator0
        (CallFunction|StartGame)))))

(fn ConstructionScript)

(fn UpdateWidgetEnum
  (params (NewWidget :type E_InWidget%20Enum :default "NewEnumerator4"))
  (Variables|Default|SetInWidget NewWidget))