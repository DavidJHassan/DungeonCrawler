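; BP_PotionTest is a potion pickup that is launched when spawned and collected by players on overlap.
; On BeginPlay the Potion component gets a random impulse, sampled from a box around the actor's world location plus an upward offset.
; On overlap, only the authority proceeds: if a Player-tagged actor's CheckForPotionMessage returns false, it calls AddPotionMessage on that actor and destroys the potion.
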(event OnComponentBeginOverlap(Potion)
  (params (OverlappedComponent :type Primitive%20Component%20Object%20Reference) (OtherActor :type Actor%20Object%20Reference) (OtherComp :type Primitive%20Component%20Object%20Reference) (OtherBodyIndex :type Integer) (bFromSweep :type Boolean) (SweepResult :type Hit%20Result%20Structure%20%28by%20ref%29))
  (Networking|SwitchHasAuthority
    (:Authority
      (if (Actor|ActorHasTag OtherActor "Player")
        (bind _haspotion (Class|INTPlayerCharacter|CheckforPotion(Message) OtherActor))
        (if (not _haspotion)
          (Class|INTPlayerCharacter|AddPotion(Message) OtherActor)
          (Actor|DestroyActor))))))

(event EventBeginPlay
  (Physics|AddImpulse (Variables|Default|GetPotion) (+ (Math|Random|RandomPointinBoundingBox (Transformation|GetActorLocation) "1000.000000,1000.000000,1000.000000") "0, 0,500.000000") "None" false))

(fn ConstructionScript)